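; Blueprint function library of shared helpers for player traces, debug output and main menu access.
; CursorRayTrace and CameraRayTrace trace the Visibility channel from the first player's cursor or camera, returning hit data; the camera trace falls back to the ray's end point on a miss.
; ErrorPrint shows red on-screen messages, and GetMainMenuWidget finds the top-level MainMenuScreen and returns it with its widget switcher.
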(fn `CameraRayTrace`
  (params (Length :type "Float (double-precision)"))
  (returns (CamRotation :type "Rotator Structure") (bBlockingHit :type Boolean) (Location :type "Vector Structure") (HitActor :type "Actor Object Reference"))
  (bind _transformcomponent (`PlayerCameraManager.TransformComponent` (`GameplayStatics.GetPlayerCameraManager` null)))
  (bind _returnvalue (`SceneComponent.K2_GetComponentLocation` _transformcomponent))
  (bind _returnvalue_2 (`SceneComponent.K2_GetComponentRotation` _transformcomponent))
  (bind _returnvalue_3 (+ _returnvalue (* (`KismetMathLibrary.GetForwardVector` _returnvalue_2) Length)))
  (bind (_outhit _returnvalue_4) (`KismetSystemLibrary.LineTraceSingle` null _returnvalue _returnvalue_3 "TraceTypeQuery1"))
  (bind (_bblockinghit _binitialoverlap _time _location _impactpoint _normal _impactnormal _physmat _hitactor) (`GameplayStatics.BreakHitResult` _outhit))
  (return _returnvalue_2 _bblockinghit (select `bool` _returnvalue_4 :`false` _returnvalue_3 :`true` _location) _hitactor))

(fn `CursorRayTrace`
  (params (bTraceComplex :type Boolean))
  (returns (bBlockingHit :type Boolean) (Location :type "Vector Structure") (HitActor :type "Actor Object Reference"))
  (bind (_bblockinghit _binitialoverlap _time _location _impactpoint _normal _impactnormal _physmat _hitactor) (`GameplayStatics.BreakHitResult` (`PlayerController.GetHitResultUnderCursorByChannel` (`GameplayStatics.GetPlayerController` null) "TraceTypeQuery1" bTraceComplex)))
  (return _bblockinghit _location _hitactor))

(fn `ErrorPrint`
  (params (InString :type String))
  (`KismetSystemLibrary.PrintString` null InString true true (struct :`R` 1.0 :`A` 1.0) 5.0))

(fn `GetMainMenuWidget`
  (returns (`AsMain Menu W` :type "/Game/Widget/MainMenu/MainMenuScreen Object Reference") (WidgetSwitcher_MM :type "WidgetSwitcher Object Reference"))
  (bind _foundwidgets (`WidgetBlueprintLibrary.GetAllWidgetsOfClass` null "/Game/Widget/MainMenu/MainMenuScreen.MainMenuScreen_C"))
  (bind _asmain_menu_screen (cast `/Game/Widget/MainMenu/MainMenuScreen` (`KismetArrayLibrary.Array_Get` _foundwidgets))
    (:`then`
      (return _asmain_menu_screen (`/Game/Widget/MainMenu/MainMenuScreen.WidgetSwitcher_MM` _asmain_menu_screen)))
    (:`CastFailed`
      (return null null))))