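; Game mode for a multiplayer truck game that assigns drivers to existing trucks and logs players joining and leaving.
; SpawnNewDriver spawns nothing: it has the given controller possess the first WheeledTruckBP without a valid instigator controller.
; Nothing in this graph calls SpawnNewDriver.
; PostLogin checks authority and casts to MyPlayerController but only prints on failure or remote, while OnLogout prints a Turkish departure message.
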(event `self.ReceiveBeginPlay`)

(event `self.K2_PostLogin`
  (params (NewPlayer :type "PlayerController Object Reference"))
  ;[1 1 1] EventOnPostLogin
  (`/Engine/EditorBlueprintResources/ActorMacros.Switch Has Authority`
    (:`Authority`
      (cast `/Game/Blueprints/MyPlayerController` NewPlayer
        (:`CastFailed`
          (`KismetSystemLibrary.PrintString` "Loign CastError"))))
    (:`Remote`
      (`KismetSystemLibrary.PrintString` "Remote"))))

(event `self.K2_OnLogout`
  (params (ExitingController :type "Controller Object Reference"))
  ;[1 1 1] EventOnLogout
  (cast `DefaultPawn` (`Controller.K2_GetPawn` ExitingController)
    (:`then`
      _)
    (:`CastFailed`
      _))
  (`KismetSystemLibrary.PrintString` "Player Oyundan Çıktı" true true (struct :`R` 0.043207 :`G` 1.0 :`A` 1.0) 10.0))

(event `SpawnNewDriver`
  (params (Controller :type "PlayerController Object Reference"))
  ;[1 1 1] SpawnNewCaptain
  (bind _outactors (`GameplayStatics.GetAllActorsOfClass` "/Game/Blueprints/WheeledTruckBP.WheeledTruckBP_C"))
  (for _array_element _outactors
    (`/Engine/EditorBlueprintResources/StandardMacros.IsValid` (`self.GetInstigatorController` _array_element)
      (:`Is Not Valid`
        (`Controller.Possess` Controller _array_element)
        (break)))))

(fn `UserConstructionScript`)