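; Game instance Blueprint that handles multiplayer sessions: hosting, searching for and joining servers.
; Hosting creates a session and opens the chosen level as a listen server, ignoring the passed Options.
; Searches are LAN-only and fill the supplied list widget with W_ServerItem entries.
; StreamLevel preloads the first PreLevels entry hidden, while session results and network or travel errors are only reported through PrintString.
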(event `StreamLevel`
  (`|ExecutionSequence`
    (:`then_0`
      (`GameplayStatics.LoadStreamLevel` (`KismetArrayLibrary.Array_Get` (`self.PreLevels`))))))

(event `HostServer`
  (params (LevelName :type Name) (PublicConnections :type Integer) (bUseLAN :type Boolean) (Options :type String))
  ;[1 1 1] Host a server
  (`CreateSessionCallbackProxy.CreateSession` (`GameplayStatics.GetPlayerController` 0) PublicConnections bUseLAN
    (:`OnSuccess`
      (`GameplayStatics.OpenLevel` LevelName true "listen"))
    (:`OnFailure`
      (`KismetSystemLibrary.PrintString` "YeniHaritaKurulamadı" true true (struct :`R` 1.0 :`A` 1.0) 4.0))))

(event `JoinToTheServer`
  (params (SearchResult :type "BlueprintSessionResult Structure (by ref)"))
  ;[1 1 1] JoinToTheServer
  (`JoinSessionCallbackProxy.JoinSession` (`GameplayStatics.GetPlayerController` 0) SearchResult
    (:`OnSuccess`
      (`KismetSystemLibrary.PrintString` "Garip :S"))
    (:`OnFailure`
      (`KismetSystemLibrary.PrintString` "Join Failed"))))

(event `SearchServers`
  (params (ServerListWidget :type "VerticalBox Object Reference"))
  ;[1 1 1] Search a server
  (bind _results (`FindSessionsCallbackProxy.FindSessions` (`GameplayStatics.GetPlayerController` 0) 10 true)
    (:`OnSuccess`
      (for _array_element _results
        (bind _returnvalue (`|CreateWidget` "/Game/Widget/SubWidgets/W_ServerItem.W_ServerItem_C" (`GameplayStatics.GetPlayerController` 0)))
        (`/Game/Widget/SubWidgets/W_ServerItem.SetWidget` _returnvalue _array_element)
        (`PanelWidget.AddChild` ServerListWidget _returnvalue))
      (`KismetSystemLibrary.PrintString` "ServersFounded"))
    (:`OnFailure`
      (`KismetSystemLibrary.PrintString` "SunucuAramaHatası" true true (struct :`R` 1.0 :`A` 1.0) 4.0))))

(event `self.HandleNetworkError`
  (params (FailureType :type "ENetworkFailure Enum" :default "NetDriverAlreadyExists") (bIsServer :type Boolean))
  ;[1 1 1] Error Displayers
  (switch `ENetworkFailure` FailureType
    (:`NetDriverAlreadyExists`
      _)
    (:`NetDriverCreateFailure`
      _)
    (:`NetDriverListenFailure`
      _)
    (:`ConnectionLost`
      _)
    (:`ConnectionTimeout`
      _)
    (:`FailureReceived`
      _)
    (:`OutdatedClient`
      _)
    (:`OutdatedServer`
      _)
    (:`PendingConnectionFailure`
      _))
  (`KismetSystemLibrary.PrintString` (`KismetStringLibrary.Concat_StrStr` "(" (`|GetEnumeratorNameAsString` FailureType) ")" "NetworkError") true true (struct :`R` 1.0 :`B` 0.14136 :`A` 1.0)))

(event `self.HandleTravelError`
  (params (FailureType :type "ETravelFailure Enum" :default "NoLevel"))
  ;[1 1 1] Error Displayers
  (switch `ETravelFailure` FailureType
    (:`NoLevel`
      _)
    (:`LoadMapFailure`
      _)
    (:`InvalidURL`
      _)
    (:`PackageMissing`
      _)
    (:`PackageVersion`
      _)
    (:`NoDownload`
      _)
    (:`TravelFailure`
      _)
    (:`CheatCommands`
      _)
    (:`PendingNetGameCreateFailure`
      _)
    (:`CloudSaveFailure`
      _)
    (:`ServerTravelFailure`
      _)
    (:`ClientTravelFailure`
      _))
  (`KismetSystemLibrary.PrintString` (`KismetStringLibrary.Concat_StrStr` "(" (`|GetEnumeratorNameAsString` FailureType) ")" "TravelError") true true (struct :`R` 1.0 :`G` 0.640718 :`A` 1.0)))