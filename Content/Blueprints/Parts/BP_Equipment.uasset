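; BP_Equipment is an equipment part actor that is set up from equipment data and can turn toward a target rotation.
; InitEquipment stores the data reference, its equipment type and socket info.
; For Dynamic types, Rotate plays a timeline that eases the actor toward the requested rotation with RInterpTo and a fixed delta.
; The TypeExecute macro gates separate execution paths for Static, OnOff and Dynamic types.
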(event `/Game/Blueprints/Parts/I_EDynamic.Rotate`
  (params (Location :type "Vector Structure") (Rotation :type "Rotator Structure"))
  (switch `/Game/Blueprints/PEquipmentTypeEnum` (`self.EqType`)
    (:`NewEnumerator2`
      (`Timeline|Timeline_0` :`NewTime` 0.0 :!via `PlayFromStart` :!label _label
        (:`Update`
          (`self.K2_SetActorRotation` (`KismetMathLibrary.RInterpTo` (`self.K2_GetActorRotation`) Rotation 0.01 5.0)))
        (:`Finished`
          (goto _label :!via `SetNewTime`))))))

(fn `InitEquipment`
  (params (PEquipment :type "/Game/Blueprints/Parts/PEquipment Object Reference") (SocketInfo :type "/Game/Blueprints/SocketInfoStr Structure"))
  (bind _output_get (set `self.PEquipmentRef` PEquipment))
  (set `self.EqType` (`/Game/Blueprints/Parts/PEquipment.EqType` _output_get))
  (set `self.SocketInfo` SocketInfo))

(fn `UserConstructionScript`)