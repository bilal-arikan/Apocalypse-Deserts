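; Sky actor that drives a day-night cycle by rotating a directional light, building on a parent sky Blueprint.
; While active, Tick adds world roll to the light, scaled by frame time and cycle speed, then updates the sun direction.
; The construction script falls back to the first DirectionalLight in the level if none is valid, and caches its intensity before running the parent script.
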(event `self.ReceiveTick`
  (params (DeltaSeconds :type "Float (single-precision)"))
  (if (`self.isActive`)
    (`self.K2_AddActorWorldRotation` (`self.Directional light actor`) (`KismetMathLibrary.MakeRotator` (* DeltaSeconds (`self.DayNightSpeed`))) false false)
    (`self.UpdateSunDirection`)))

(fn `UserConstructionScript`
  (`/Engine/EditorBlueprintResources/StandardMacros.IsValid` (`self.Directional light actor`)
    (:`Is Valid`
      _)
    (:`Is Not Valid`
      (bind _outactors (`GameplayStatics.GetAllActorsOfClass` "/Script/Engine.DirectionalLight"))
      (bind _output_get (set `self.Directional light actor` (`KismetArrayLibrary.Array_Get` _outactors)))))
  (set `self.intensity` (`LightComponentBase.Intensity` (`Light.LightComponent` _output_get)))
  (`parent.UserConstructionScript`))